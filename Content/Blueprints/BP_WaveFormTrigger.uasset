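; BP_WaveFormTrigger is a trigger actor that switches the waveform in the sound analyzer when another actor overlaps it.
; On BeginPlay it labels its text component with "Form" plus its Number.
; On overlap it passes that Number to the SoundAnalyzer's ChangeWaveForm, first finding and caching the first SoundAnalyzer in the level if none is set.
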(event `self.ReceiveBeginPlay`
  (bind _output_get (set `self.BoxText` (`KismetTextLibrary.Conv_StringToText` (`KismetStringLibrary.Concat_StrStr` "Form " (`KismetStringLibrary.Conv_IntToString` (`self.Number`))))))
  (`TextRenderComponent.K2_SetText` (`self.Text `) _output_get))

(event `self.ReceiveActorBeginOverlap`
  (params (OtherActor :type "Actor Object Reference"))
  (`/Engine/EditorBlueprintResources/StandardMacros.IsValid` (`self.SoundAnalyzerRef`)
    (:`Is Valid`
      _)
    (:`Is Not Valid`
      (bind _outactors (`GameplayStatics.GetAllActorsOfClass` "/Game/Blueprints/SoundAnalyzer.SoundAnalyzer_C"))
      (set `self.SoundAnalyzerRef` (`|GetArrayItem` _outactors))))
  (`/Game/Blueprints/SoundAnalyzer.ChangeWaveForm` (`self.SoundAnalyzerRef`) (`self.Number`)))

(fn `UserConstructionScript`)