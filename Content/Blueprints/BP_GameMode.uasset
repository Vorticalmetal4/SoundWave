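; Game mode that sets up a sound wave visualisation when play begins.
; It spawns a row of BP_WavePoint actors evenly spaced along Y from WavePointLocation, with the count driven by SoundWaveSize.
; Each point receives its index and records its spawn location as StartPoint, then a single SoundAnalyzer actor is spawned at the world origin.
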(event `self.ReceiveBeginPlay`
  (for _index (range (+ (`self.SoundWaveSize`) 1))
    (bind _returnvalue (`|SpawnActorFromClass` "/Game/Blueprints/BP_WavePoint.BP_WavePoint_C" (`KismetMathLibrary.MakeTransform` (+ (`KismetMathLibrary.MakeVector` 0.0 (`KismetMathLibrary.Conv_IntToDouble` (* _index 55))) (`self.WavePointLocation`))) "Undefined" "OverrideRootScale" null null))
    (set `/Game/Blueprints/BP_WavePoint.index` _index _returnvalue)
    (set `/Game/Blueprints/BP_WavePoint.StartPoint` (`self.K2_GetActorLocation` _returnvalue) _returnvalue))
  (`|SpawnActorFromClass` "/Game/Blueprints/SoundAnalyzer.SoundAnalyzer_C" (`KismetMathLibrary.MakeTransform` (0.0 0.0 0.0)) "Undefined" "OverrideRootScale" null null))

(fn `UserConstructionScript`)