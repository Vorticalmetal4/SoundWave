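; Actor that drives an audio-reactive visualizer by playing a sound and feeding its spectrum to BP_WavePoint actors in the level.
; The construction script gathers all wave points, and BeginPlay starts playback and binds the playback-percent callback.
; Each callback converts percent to time, samples channel 0 normalized Constant-Q bands, and passes each band to the same-indexed point.
; ChangeWaveForm selects which of three point forms receives the values.
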(event `self.ReceiveBeginPlay`
  (bind _sound (`self.Sound`))
  (`AudioComponent.SetSound` (`self.Audio`) _sound)
  (set `self.Duration` (`SoundBase.Duration` _sound))
  (add `AudioComponent.OnAudioPlaybackPercent` (`self.Audio`) (delegate `PlaybackPercent`))
  (`AudioComponent.Play` (`self.Audio`) 0.0))

(event `PlaybackPercent`
  (params (PlayingSoundWave :type "SoundWave Object Reference") (PlaybackPercent :type "Float (single-precision)"))
  (set `self.PlayedTime` (* PlaybackPercent (`self.Duration`)))
  (for (_array_element _array_index) (`ConstantQNRT.GetNormalizedChannelConstantQAtTime` (`self.Constant`) (`self.PlayedTime`) 0)
    (bind _output (`|GetArrayItem` (`self.WavePoints`) _array_index))
    (`/Engine/EditorBlueprintResources/StandardMacros.IsValid` _output
      (:`Is Valid`
        (switch `int` (`self.Form`)
          (:`0`
            (`/Game/Blueprints/BP_WavePoint.FirstForm` _output _array_element))
          (:`1`
            (`/Game/Blueprints/BP_WavePoint.Second Form` _output _array_element))
          (:`2`
            (`/Game/Blueprints/BP_WavePoint.ThirdForm` _output _array_element)))))))

(fn `ChangeWaveForm`
  (params (FormNumber :type Integer))
  (set `self.Form` FormNumber))

(fn `UserConstructionScript`
  (bind _outactors (`GameplayStatics.GetAllActorsOfClass` "/Game/Blueprints/BP_WavePoint.BP_WavePoint_C"))
  (set `self.WavePoints` _outactors))