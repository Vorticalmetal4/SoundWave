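; BP_WavePoint is a single point in a wave display that poses itself in one of three forms from a ConstantQ value.
; FirstForm stretches its height at StartPoint, SecondForm lifts it at unit scale, and ThirdForm stretches a thinner shape at a fixed raised offset.
; The event graph and construction script are empty, so the form functions rely on outside callers to supply the value.
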(fn `FirstForm`
  (params (ConstantQ :type "Float (double-precision)"))
  (`self.SetActorScale3D` (`KismetMathLibrary.MakeVector` 1.0 1.0 (* ConstantQ 25.0)))
  (`self.K2_SetActorLocation` (`self.StartPoint`)))

(fn `Second Form`
  (params (ConstantQ :type "Float (double-precision)"))
  (`self.K2_SetActorLocation` (`KismetMathLibrary.MakeVector` (.x (`self.StartPoint`)) (.y (`self.StartPoint`)) (+ (* ConstantQ 600.0) (.z (`self.StartPoint`)))))
  (`self.SetActorScale3D` (1.0 1.0 1.0)))

(fn `ThirdForm`
  (params (ConstantQ :type "Float (double-precision)"))
  (bind (_startpoint_x _startpoint_y _startpoint_z) (`KismetMathLibrary.BreakVector` (`self.StartPoint`)))
  (`self.SetActorScale3D` (`KismetMathLibrary.MakeVector` 0.2 0.2 (* ConstantQ 10.0)))
  (`self.K2_SetActorLocation` (`KismetMathLibrary.MakeVector` _startpoint_x _startpoint_y (+ _startpoint_z 200.0))))

(fn `UserConstructionScript`)